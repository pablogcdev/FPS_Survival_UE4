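; FPS game mode that runs zombie rounds, starting the first on BeginPlay after caching the game state and all EnemySpawner actors.
; A new round plays a sting, waits, increments the round on the game state, then starts a looping timer.
; Each tick spawns a zombie at a random spawner until the game state's zombie count reaches the round's target, then clears the timer.
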(event `self.ReceiveBeginPlay`
  (bind _asfps_game_state (cast `/Game/Blueprints/FPS_GameState` (`GameplayStatics.GetGameState`)))
  (set `self.GameState_Ref` _asfps_game_state)
  (bind _outactors (`GameplayStatics.GetAllActorsOfClass` "/Game/Blueprints/Actors/EnemySpawner.EnemySpawner_C"))
  (set `self.EnemySpawners` _outactors)
  (`self.StartNewRound`))

(event `StartNewRound`
  (`GameplayStatics.PlaySound2D` "/Game/Sounds/Stingers/wav/sw_Sting_Respawn.sw_Sting_Respawn" 1.0 1.0 0.0 null null)
  (`KismetSystemLibrary.Delay` 10.0)
  (`/Game/Blueprints/FPS_GameState.IncreaseRound` (`self.GameState_Ref`))
  (bind _returnvalue (`KismetSystemLibrary.K2_SetTimerDelegate` (delegate `SpawnZombies`) 2.5 true)))

(event `SpawnZombies`
  (bind _gamestate_ref (`self.GameState_Ref`))
  (bind _enemyspawners (`self.EnemySpawners`))
  (if (< (`/Game/Blueprints/FPS_GameState.NumberOfZombies` _gamestate_ref) (`/Game/Blueprints/FPS_GameState.NumberOfZombiesToSpawn` _gamestate_ref))
    (`/Game/Blueprints/Actors/EnemySpawner.SpawnZombie` (`|GetArrayItem` _enemyspawners (`KismetMathLibrary.RandomIntegerInRange` 0 (- (`KismetArrayLibrary.Array_Length` _enemyspawners) 1))))
    (else
      (`KismetSystemLibrary.K2_ClearAndInvalidateTimerHandle` (stale `StartNewRound` _returnvalue)))))

(fn `UserConstructionScript`)