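; FPS_GameState tracks the round number and zombie count for a wave-based zombie shooter.
; On BeginPlay it caches the FPS game mode and player character.
; IncreaseRound advances the round, scales the zombie count linearly with a clamped cap and pushes both values to the player's HUD.
; CheckIfRoundIsOver asks the game mode to start a new round once the zombie count reaches zero.
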(event `self.ReceiveBeginPlay`
  (bind _asfps_game_mode (cast `/Game/Blueprints/FPS_GameMode` (`GameplayStatics.GetGameMode`)))
  (set `self.GameMode_Ref` _asfps_game_mode)
  (bind _asfps_character (cast `/Game/Blueprints/FPS_Character` (`GameplayStatics.GetPlayerPawn` 0)))
  (set `self.Player_Ref` _asfps_character))

(fn `CheckIfRoundIsOver`
  (if (<= (`self.NumberOfZombiesToSpawn`) 0)
    (`/Game/Blueprints/FPS_GameMode.StartNewRound` (`self.GameMode_Ref`))))

(fn `IncreaseRound`
  (bind _currentround (`self.CurrentRound`))
  (`/Engine/EditorBlueprintResources/StandardMacros.IncrementInt` _currentround
    (:`  `
      (bind _output_get (set `self.NumberOfZombiesToSpawn` (`KismetMathLibrary.Clamp` (`KismetMathLibrary.Round` (+ (* _currentround 1.5) 9.0)) 0 150)))
      (`/Game/Blueprints/UMG/UI_RoundNumber.UpdateData` (`/Game/Blueprints/UMG/MainHUD.UI_RoundNumber` (`/Game/Blueprints/FPS_Character.MainHUDRef` (`self.Player_Ref`))) (`self.CurrentRound`) _output_get))))

(fn `UserConstructionScript`)