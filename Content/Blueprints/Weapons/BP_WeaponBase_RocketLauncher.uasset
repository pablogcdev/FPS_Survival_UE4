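; Rocket launcher weapon Blueprint that extends a parent weapon's startup and fire behavior.
; On BeginPlay it pulls its rocket launcher ammo data from the FPS game instance.
; Firing runs the parent logic, then plays the gun mesh's fire animation and a world camera shake centered on the weapon.
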(event `self.ReceiveBeginPlay`
  (`parent.ReceiveBeginPlay`)
  (bind _asfps_game_instance (cast `/Game/Blueprints/FPS_GameInstance` (`GameplayStatics.GetGameInstance`)))
  (set `self.AmmoData` (`/Game/Blueprints/FPS_GameInstance.RocketLauncherAmmoData` _asfps_game_instance)))

(event `self.Weapon Fire`
  (params (FireType :type "/Game/Blueprints/Enums/FireType Enum" :default "NewEnumerator0"))
  (`parent.Weapon Fire` FireType)
  (`SkeletalMeshComponent.PlayAnimation` (`self.GunMesh`) "/Game/MilitaryWeapSilver/Weapons/Animations/Fire_RocketLauncher_W.Fire_RocketLauncher_W" false)
  (`GameplayStatics.PlayWorldCameraShake` "/Game/Blueprints/CameraShakes/RocketLauncher_CameraShake.RocketLauncher_CameraShake_C" (`self.K2_GetActorLocation`) 0.0 500.0))

(fn `UserConstructionScript`
  (`parent.UserConstructionScript`))